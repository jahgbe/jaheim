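; BP_Key is a key actor meant to appear and become collidable once no B_Print actors, treated as targets, remain.
; Every Tick it gathers all B_Print actors, uses the index returned by an array Add as their count, and toggles mesh visibility and actor collision from the result.
; BeginPlay caches the first-person character, but the collision overlap check leads to no action, so pickup is unimplemented.
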(event `self.ReceiveBeginPlay`
  ; Setup
  (bind _asbp_first_person_character (cast `/Game/StarterContent/FirstPerson/Blueprints/BP_FirstPersonCharacter` (`GameplayStatics.GetPlayerCharacter` 0)))
  (set `self. BP_FirstPersonCharacter` _asbp_first_person_character))

(event `self.ReceiveTick`
  (params (DeltaSeconds :type "Float (single-precision)"))
  ; Key Visibility
  (bind _outactors (`GameplayStatics.GetAllActorsOfClass` "/Game/MyContent/Blueprints/B_Print.B_Print_C"))
  (bind _returnvalue (`KismetArrayLibrary.Array_Add` _outactors))
  (bind _output_get (set `self.AllTargetsDestroyed` (<= _returnvalue 0)))
  (`SceneComponent.SetVisibility` (`self.SM_Key`) _output_get true)
  (`self.SetActorEnableCollision` _output_get))

(event `self.Collision.OnComponentBeginOverlap`
  (params (OverlappedComponent :type "PrimitiveComponent Object Reference") (OtherActor :type "Actor Object Reference") (OtherComp :type "PrimitiveComponent Object Reference") (OtherBodyIndex :type Integer) (bFromSweep :type Boolean) (SweepResult :type "HitResult Structure (by ref)"))
  (if (and (== OtherActor null) (`self.AllTargetsDestroyed`))
    _))

(fn `UserConstructionScript`)